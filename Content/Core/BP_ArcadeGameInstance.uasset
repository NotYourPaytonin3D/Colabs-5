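; Arcade game instance that stores the character picks for two players and serves character data from the DT_Characters data table.
; Picks are saved as slot indices, which map to the table's row names by position.
; Lookups check the slot is valid and return the row with a Found flag.
; GetPickedCharacter resolves player index 0 to P1's pick and any other index to P2's.
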(fn `GetCharacter`
  (params (Slot :type Integer))
  (returns (Character :type "/Game/Core/Characters/S_Character Structure") (Found :type Boolean))
  (bind _outrownames (`DataTableFunctionLibrary.GetDataTableRowNames` "/Game/Core/Characters/DT_Characters.DT_Characters"))
  (if (`KismetArrayLibrary.Array_IsValidIndex` _outrownames Slot)
    (bind _returnvalue (`|GetDataTableRow` "/Game/Core/Characters/DT_Characters.DT_Characters" (`|GetArrayItem` _outrownames Slot))
      (:`then`
        (return _returnvalue true))
      (:`RowNotFound`
        (return (struct) false)))
    (else
      (return (struct) false))))

(fn `GetCharacterCount`
  (returns (Count :type Integer))
  (bind _outrownames (`DataTableFunctionLibrary.GetDataTableRowNames` "/Game/Core/Characters/DT_Characters.DT_Characters"))
  (return (`KismetArrayLibrary.Array_Length` _outrownames)))

(fn `GetPickedCharacter`
  (params (PlayerIndex :type Integer))
  (returns (Character :type "/Game/Core/Characters/S_Character Structure") (Found :type Boolean))
  (bind (_character _found) (`self.GetCharacter` (`KismetMathLibrary.SelectInt` (`self.P1_Character`) (`self.P2_Character`) (== PlayerIndex 0))))
  (return _character _found))

(fn `SetPicks`
  (params (P1 :type Integer) (P2 :type Integer))
  (set `self.P1_Character` P1)
  (set `self.P2_Character` P2))