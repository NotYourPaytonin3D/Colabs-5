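; BP_FightCamera is a side-on camera that keeps both fighters framed during a fight.
; On BeginPlay it takes the first two BP_Fighter actors in the level and sets a fixed rotation.
; Each tick, while both are valid, it eases toward their midpoint on X at constant height, pulling back along Y in proportion to their separation within clamped limits.
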(event `self.ReceiveBeginPlay`
  (bind _outactors (`GameplayStatics.GetAllActorsOfClass` "/Game/Fighter/BP_Fighter.BP_Fighter_C"))
  (set `self.A` (`|GetArrayItem` _outactors))
  (set `self.B` (`|GetArrayItem` _outactors 1))
  (`self.K2_SetActorRotation` (struct :`Pitch` -5.0 :`Yaw` -90.0)))

(event `self.ReceiveTick`
  (params (DeltaSeconds :type "Float (single-precision)"))
  (bind _returnvalue_x (`KismetMathLibrary.BreakVector` (`self.K2_GetActorLocation` (`self.B`))))
  (bind _returnvalue_x_2 (`KismetMathLibrary.BreakVector` (`self.K2_GetActorLocation` (`self.A`))))
  (if (and (`KismetSystemLibrary.IsValid` (`self.A`)) (`KismetSystemLibrary.IsValid` (`self.B`)))
    (`self.K2_SetActorLocation` (`KismetMathLibrary.VInterpTo` (`self.K2_GetActorLocation`) (`KismetMathLibrary.MakeVector` (/ (+ _returnvalue_x_2 _returnvalue_x) 2.0) (`KismetMathLibrary.FClamp` (+ (* (`KismetMathLibrary.Abs` (- _returnvalue_x_2 _returnvalue_x)) 1.4) 870.0) 1050.0 1900.0) 160.0) DeltaSeconds 5.0))))

(fn `UserConstructionScript`)