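; BP_FightController is the player controller for a local two-player fighting game, driving both fighters from one controller.
; On BeginPlay it finds the BP_Fighter actors by PlayerIndex, links them as opponents, adds the IMC_Fight mapping context, switches view to BP_FightCamera and creates the fight HUD.
; Separate P1 and P2 Enhanced Input actions forward move, attack and jump to the matching fighter.
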(event `self.ReceiveBeginPlay`
  (bind _outactors (`GameplayStatics.GetAllActorsOfClass` "/Game/Fighter/BP_Fighter.BP_Fighter_C"))
  (for _array_element _outactors
    (switch `int` (`/Game/Fighter/BP_Fighter.PlayerIndex` _array_element)
      (:`0`
        (set `self.P1` _array_element))
      (:`1`
        (set `self.P2` _array_element))))
  (set `/Game/Fighter/BP_Fighter.Opponent` (`self.P2`) (`self.P1`))
  (set `/Game/Fighter/BP_Fighter.Opponent` (`self.P1`) (`self.P2`))
  (`EnhancedInputSubsystemInterface.AddMappingContext` (pcsubsystem `EnhancedInputLocalPlayerSubsystem` self) "/Game/Input/IMC_Fight.IMC_Fight" 0 (struct))
  (bind _returnvalue (`GameplayStatics.GetActorOfClass` "/Game/Core/Fight/BP_FightCamera.BP_FightCamera_C"))
  (`self.SetViewTargetWithBlend` _returnvalue)
  (bind _returnvalue_2 (`|CreateWidget` "/Game/UI/WBP_FightHUD.WBP_FightHUD_C" self (`self.P1`) (`self.P2`)))
  (bind _output_get (set `self.Hud` _returnvalue_2))
  (`UserWidget.AddToViewport` _output_get 0)
  (`WidgetBlueprintLibrary.SetInputMode_GameOnly` self))

(event `EnhancedInput|/Game/Input/Actions/IA_P1_Move`
  (params (ActionValue :type "Float (double-precision)") (ElapsedSeconds :type "Float (double-precision)") (TriggeredSeconds :type "Float (double-precision)") (InputAction :type "InputAction Object Reference" :default "/Game/Input/Actions/IA_P1_Move.IA_P1_Move"))
  ; P1 Actions
  (:`Triggered`
    (`/Game/Fighter/BP_Fighter.SetMoveInput` (`self.P1`) ActionValue))
  (:`Completed`
    (`/Game/Fighter/BP_Fighter.SetMoveInput` (`self.P1`) 0.0)))

(event `EnhancedInput|/Game/Input/Actions/IA_P2_Move`
  (params (ActionValue :type "Float (double-precision)") (ElapsedSeconds :type "Float (double-precision)") (TriggeredSeconds :type "Float (double-precision)") (InputAction :type "InputAction Object Reference" :default "/Game/Input/Actions/IA_P2_Move.IA_P2_Move"))
  ; P2 Actions
  (:`Triggered`
    (`/Game/Fighter/BP_Fighter.SetMoveInput` (`self.P2`) ActionValue))
  (:`Completed`
    (`/Game/Fighter/BP_Fighter.SetMoveInput` (`self.P2`) 0.0)))

(event `EnhancedInput|/Game/Input/Actions/IA_P1_Attack`
  (params (ActionValue :type Boolean) (ElapsedSeconds :type "Float (double-precision)") (TriggeredSeconds :type "Float (double-precision)") (InputAction :type "InputAction Object Reference" :default "/Game/Input/Actions/IA_P1_Attack.IA_P1_Attack"))
  ; P1 Actions
  (:`Started`
    (`/Game/Fighter/BP_Fighter.Attack` (`self.P1`))))

(event `EnhancedInput|/Game/Input/Actions/IA_P2_Attack`
  (params (ActionValue :type Boolean) (ElapsedSeconds :type "Float (double-precision)") (TriggeredSeconds :type "Float (double-precision)") (InputAction :type "InputAction Object Reference" :default "/Game/Input/Actions/IA_P2_Attack.IA_P2_Attack"))
  ; P2 Actions
  (:`Started`
    (`/Game/Fighter/BP_Fighter.Attack` (`self.P2`))))

(event `EnhancedInput|/Game/Input/Actions/IA_P1_Jump`
  (params (ActionValue :type Boolean) (ElapsedSeconds :type "Float (double-precision)") (TriggeredSeconds :type "Float (double-precision)") (InputAction :type "InputAction Object Reference" :default "/Game/Input/Actions/IA_P1_Jump.IA_P1_Jump"))
  ; P1 Actions
  (:`Triggered`
    (`/Game/Fighter/BP_Fighter.DoJump` (`self.P1`))))

(event `EnhancedInput|/Game/Input/Actions/IA_P2_Jump`
  (params (ActionValue :type Boolean) (ElapsedSeconds :type "Float (double-precision)") (TriggeredSeconds :type "Float (double-precision)") (InputAction :type "InputAction Object Reference" :default "/Game/Input/Actions/IA_P2_Jump.IA_P2_Jump"))
  ; P2 Actions
  (:`Triggered`
    (`/Game/Fighter/BP_Fighter.DoJump` (`self.P2`))))

(fn `UserConstructionScript`)