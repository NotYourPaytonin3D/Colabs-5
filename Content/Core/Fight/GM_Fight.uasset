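; GM_Fight is the game mode for a fight match, handling the end of the match when a fighter is knocked out.
; FighterKO latches MatchOver so only the first KO counts, then derives the winning player from the loser's PlayerIndex.
; It shows the winner through the HUD of the first player's BP_FightController, then reloads the current level after a short delay.
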(event `FighterKO`
  (params (Loser :type "/Game/Fighter/BP_Fighter Object Reference"))
  (if (not (`self.MatchOver`))
    (set `self.MatchOver` true)
    (bind _asbp_fight_controller (cast `/Game/Core/Fight/BP_FightController` (`GameplayStatics.GetPlayerController` 0)))
    (`/Game/Ui/WBP_FightHUD.ShowWinner` (`/Game/Core/Fight/BP_FightController.Hud` _asbp_fight_controller) (`KismetMathLibrary.SelectText` "PLAYER 2 WINS" "PLAYER 1 WINS" (== (`/Game/Fighter/BP_Fighter.PlayerIndex` Loser) 0)))
    (`KismetSystemLibrary.Delay` 3.0)
    (bind _returnvalue (`GameplayStatics.GetCurrentLevelName` true))
    (`GameplayStatics.OpenLevel` (`KismetStringLibrary.Conv_StringToName` _returnvalue))))

(fn `UserConstructionScript`)