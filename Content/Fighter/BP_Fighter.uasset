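; 2D flipbook fighter character for a versus fight, loading its sprites, stats and tint from the character picked in the game instance.
; It moves along X, faces its opponent, jumps, blocks by holding back, and attacks with a delayed sphere overlap that triggers TakeHit.
; Zero health causes a timed knockdown with full-health recovery, until the knockdown limit reports a KO to GM_Fight.
; State flags gate actions and select the flipbook each tick.
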(event `self.ReceiveBeginPlay`
  (`self.ApplyCharacter`)
  (set `self.Health` (`self.MaxHealth`)))

(event `self.ReceiveTick`
  (params (DeltaSeconds :type "Float (single-precision)"))
  (`|ExecutionSequence`
    (:`then_0`
      (if (`self.CanAct`)
        (`self.AddMovementInput` (1.0 0.0 0.0) (`self.MoveInput`))))
    (:`then_1`
      (`self.FaceOpponent`))
    (:`then_2`
      (`self.UpdateAnimation`))))

(event `DoJump`
  (if (`self.CanPlayerDoSomething`)
    (`self.Jump`)))

(event `TakeHit`
  (params (Damage :type "Float (double-precision)") (Direction :type "Float (double-precision)"))
  (if (or (`self.IsDead`) (`self.IsKnockedDown`))
    _
    (elif (`self.IsBlocking`)
      (`self.K2_AddActorWorldOffset` (* Direction (20.0 0.0 0.0)) true)
      (else
        (set `self.Health` (`KismetMathLibrary.FMax` (- (`self.Health`) Damage)))
        (set `self.IsAttacking` false)
        (set `self.IsHurt` true)
        (`self.LaunchCharacter` (`KismetMathLibrary.MakeVector` (* Direction (`self.KnockBack`)) 0.0 250.0) true true)
        (if (<= (`self.Health`) 0.0)
          (`self.Die`)
          (else
            (`KismetSystemLibrary.RetriggerableDelay` 0.35)
            (set `self.IsHurt` false)))))))

(event `Die`
  ;[0.12 0.12 0.12] Health ran out: that is one knockdown.
  ; On knockdown number KnockdownsToLose (2) the fighter is out and GM_Fight shows who won.
  ; Before that it stays down for KnockdownTime, then gets up with full health
  (set `self.Knockdowns` (+ (`self.Knockdowns`) 1))
  (`self.ShowKnockdownsOnHud`)
  (`self.SetMoveInput` 0.0)
  (if (>= (`self.Knockdowns`) (`self.KnockdownsToLose`))
    (set `self.IsDead` true)
    (bind _asgm_fight (cast `/Game/Core/Fight/GM_Fight` (`GameplayStatics.GetGameMode`)))
    (`/Game/Core/Fight/GM_Fight.FighterKO` _asgm_fight self)
    (else
      (set `self.IsKnockedDown` true)
      (`KismetSystemLibrary.Delay` (`self.KnockdownTime`))
      (set `self.Health` (`self.MaxHealth`))
      (set `self.IsHurt` false)
      (set `self.IsKnockedDown` false))))

(event `Attack`
  ; Attacks
  (if (`self.CanPlayerDoSomething`)
    (set `self.IsAttacking` true)
    (`KismetSystemLibrary.Delay` 0.15)
    (if (`self.IsAttacking`)
      (`self.CheckHit`)
      (`KismetSystemLibrary.Delay` 0.35)
      (set `self.IsAttacking` false))))

(fn `ApplyCharacter`
  (bind _asbp_arcade_game_instance (cast `/Game/Core/BP_ArcadeGameInstance` (`GameplayStatics.GetGameInstance`)))
  (bind (_character _found) (`/Game/Core/BP_ArcadeGameInstance.GetPickedCharacter` _asbp_arcade_game_instance (`self.PlayerIndex`)))
  (if _found
    (`self.UseSprites` _character)
    (`self.UseStats` _character)))

(fn `CanAct`
  (returns (Result :type Boolean))
  (if (`KismetSystemLibrary.IsValid` (`self.Opponent`))
    (return (and (not (`self.IsAttacking`)) (not (`self.IsHurt`)) (not (`self.IsDead`)) (not (`/Game/Fighter/BP_Fighter.IsDead` (`self.Opponent`))) (not (`self.IsKnockedDown`))))
    (else
      (return false))))

(fn `CheckHit`
  (bind _returnvalue (+ (`self.K2_GetActorLocation`) (* (`self.FacingSign`) (70.0 0.0 10.0))))
  (`KismetSystemLibrary.DrawDebugSphere` _returnvalue 100.0 12 (struct :`R` 1.0 :`G` 1.0 :`B` 1.0 :`A` 1.0) 0.5)
  (bind _outactors (`KismetSystemLibrary.SphereOverlapActors` _returnvalue 50.0 (`|MakeArray` "ObjectTypeQuery3" :!type "EObjectTypeQuery Enum") "BP_Fighter_C" (`|MakeArray` self :!type "Actor Object Reference")))
  (for _array_element _outactors
    (bind _asbp_fighter (cast `/Game/Fighter/BP_Fighter` _array_element))
    (`self.TakeHit` _asbp_fighter (`self.AttaclDamage`) (`self.FacingSign`))))

(fn `FaceOpponent`
  (bind _returnvalue_x (`KismetMathLibrary.BreakVector` (`self.K2_GetActorLocation`)))
  (bind _returnvalue_x_2 (`KismetMathLibrary.BreakVector` (`SceneComponent.K2_GetComponentLocation` (`PaperCharacter.Sprite` (`self.Opponent`)))))
  (if (`self.CanAct`)
    (set `self.FacingSign` (`KismetMathLibrary.SelectFloat` 1.0 -1.0 (> _returnvalue_x_2 _returnvalue_x)))
    (`SceneComponent.SetRelativeScale3D` (`self.Sprite`) (`KismetMathLibrary.MakeVector` (* (`self.FacingSign`) 3.0) 3.0 3.0))))

(fn `IsBlocking`
  (returns (Result :type Boolean))
  (return (and (not (`self.IsAttacking`)) (not (`self.IsHurt`)) (not (`self.IsDead`)) (not (`NavMovementInterface.IsFalling` (`self.CharacterMovement`))) (`self.IsHoldingBack`))))

(fn `IsHoldingBack`
  (returns (Result :type Boolean))
  (return (< (* (`self.MoveInput`) (`self.FacingSign`)) -0.1)))

(fn `SetFlipbook`
  (params (Wanted :type "PaperFlipbook Object Reference"))
  (bind _sprite (`self.Sprite`))
  (if (!= (`PaperFlipbookComponent.GetFlipbook` (`self.Sprite`)) Wanted)
    (`PaperFlipbookComponent.SetFlipbook` (`self.Sprite`) Wanted)
    (if (and (!= Wanted (`self.DeathFlipbook`)) (!= Wanted (`self.AttackFlipbook`)))
      (`PaperFlipbookComponent.SetLooping` _sprite true)
      (else
        (`PaperFlipbookComponent.SetLooping` _sprite false)))
    (`PaperFlipbookComponent.PlayFromStart` (`self.Sprite`))))

(fn `SetMoveInput`
  (params (Value :type "Float (double-precision)"))
  (set `self.MoveInput` Value))

(fn `ShowKnockdownsOnHud`
  ;[0.12 0.12 0.12] The fight HUD lives on BP_FightController.
  ; Ask it to redraw the knockdown markers
  (bind _asbp_fight_controller (cast `/Game/Core/Fight/BP_FightController` (`GameplayStatics.GetPlayerController` 0)))
  (bind _hud (`/Game/Core/Fight/BP_FightController.Hud` _asbp_fight_controller))
  (if (`KismetSystemLibrary.IsValid` _hud)
    (`/Game/UI/WBP_FightHUD.RefreshKnockdowns` _hud)))

(fn `UpdateAnimation`
  (locals (Wanted :type "PaperFlipbook Object Reference"))
  (bind (_returnvalue_x _returnvalue_y _returnvalue_z) (`KismetMathLibrary.BreakVector` (`self.GetVelocity`)))
  (bind _returnvalue_x_2 (`KismetMathLibrary.BreakVector` (`self.GetVelocity`)))
  (`|ExecutionSequence`
    (:`then_0`
      (if (or (`self.IsDead`) (`self.IsKnockedDown`))
        (set `local.Wanted` (`self.DeathFlipbook`))
        (elif (`self.IsHurt`)
          (set `local.Wanted` (`self.HitFlipbook`))
          (elif (`self.IsAttacking`)
            (set `local.Wanted` (`self.AttackFlipbook`))
            (elif (`NavMovementInterface.IsFalling` (`self.CharacterMovement`))
              (if (> _returnvalue_z 0.0)
                (set `local.Wanted` (`self.JumpFlipbook`))
                (else
                  (set `local.Wanted` (`self.FallFlipbook`))))
              (elif (> (`KismetMathLibrary.Abs` _returnvalue_x_2) 10.0)
                (set `local.Wanted` (`self.RunFlipbook`))
                (else
                  (set `local.Wanted` (`self.IdleFlipbook`)))))))))
    (:`then_1`
      (`self.SetFlipbook` (`local.Wanted`)))
    (:`then_2`
      (`KismetSystemLibrary.DrawDebugString` (`SceneComponent.K2_GetComponentLocation` (`self.DebugTextLocation`)) (`KismetStringLibrary.Concat_StrStr` (`KismetSystemLibrary.GetDisplayName` (`local.Wanted`)) " By Player" (`KismetSystemLibrary.GetDisplayName` self)) null))))

(fn `UserConstructionScript`)

(fn `UseSprites`
  (params (Character :type "/Game/Core/Characters/S_Character Structure"))
  (bind (_displayname _portrait _idleflipbook _runflipbook _jumpflipbook _fallflipbook _attackflipbook _hitflipbook _deathflipbook) (break `/Game/Core/Characters/S_Character` Character))
  (set `self.IdleFlipbook` _idleflipbook)
  (set `self.RunFlipbook` _runflipbook)
  (set `self.JumpFlipbook` _jumpflipbook)
  (set `self.FallFlipbook` _fallflipbook)
  (set `self.AttackFlipbook` _attackflipbook)
  (set `self.HitFlipbook` _hitflipbook)
  (set `self.DeathFlipbook` _deathflipbook))

(fn `UseStats`
  (params (Character :type "/Game/Core/Characters/S_Character Structure"))
  (bind (_displayname _portrait _idleflipbook _runflipbook _jumpflipbook _fallflipbook _attackflipbook _hitflipbook _deathflipbook _maxhealth _attackdamage _tint) (break `/Game/Core/Characters/S_Character` Character))
  (set `self.MaxHealth` _maxhealth)
  (set `self.AttaclDamage` _attackdamage)
  (`PaperFlipbookComponent.SetSpriteColor` (`self.Sprite`) _tint))